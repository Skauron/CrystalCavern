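; BP_WinVolume is a volume that completes the level when the player overlaps it and no BP_Crystal actors remain in the world.
; On overlap it filters for the player, then counts crystals with GetAllActorsOfClass.
; Completion finds the current level's name in the ordered LevelNames array and opens the next entry by name, or quits the game if it is the last.
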(event EventBeginPlay)

(event Collision|EventActorBeginOverlap
  (params (OtherActor :type Actor%20Object%20Reference))
  (Utilities|IsPlayer OtherActor
    (:Is%20Player
      (if (not (CallFunction|AnyCrystalsRemaining))
        (LevelManangement|CompleteLevel)))))

(fn ConstructionScript)

(fn AnyCrystalsRemaining
  (bind _outactors (Actor|GetAllActorsOfClass "/Game/Blueprints/Actors/Collectables/BP_Crystal.BP_Crystal_C"))
  (return (> (Utilities|Array|Length _outactors) 0)))

(fn CompleteLevel
  (if (LevelManangement|IsFinalLevel)
    (Game|QuitGame 0 "Quit" false)
    (else
      (LevelManangement|LoadNextLevel))))

(fn GetCurrentLevelIndex
  (bind _returnvalue (Game|GetCurrentLevelName true))
  (return (Utilities|Array|FindItem (Variables|Default|GetLevel%20Names) (Utilities|String|StringToName _returnvalue))))

(fn IsFinalLevel
  (return (== (Utilities|Array|LastIndex (Variables|Default|GetLevel%20Names)) (LevelManangement|GetCurrentLevelIndex))))

(fn LoadNextLevel
  (Game|OpenLevel(byName) (LevelManangement|GetNextLevelName)))

(fn GetNextLevelName
  (return (Utilities|Array|Get(acopy) (Variables|Default|GetLevel%20Names) (+ 1 (LevelManangement|GetCurrentLevelIndex)))))