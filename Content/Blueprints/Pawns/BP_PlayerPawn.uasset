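; Player pawn that moves by applying physics torque to its mesh and restarts the level when it takes any damage.
; On BeginPlay it adds the game's Enhanced Input mapping context and fades the camera in.
; Move input drives acceleration-based torque on the X and Y axes.
; The Restart Level graph uses DoOnce to fade the camera out a single time, then reloads the current level by name after a matching delay.
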(event Input|EnhancedActionEvents|EnhancedInputActionIA_Move
  (params (ActionValue :type Vector%202D%20Structure) (ElapsedSeconds :type Float%20%28double-precision%29) (TriggeredSeconds :type Float%20%28double-precision%29) (InputAction :type Input%20Action%20Object%20Reference :default "/Game/EnhancedInput/IA_Move.IA_Move"))
  (bind _acceleration (Variables|Default|GetAcceleration))
  (Class|PrimitiveComponent|AddTorqueinRadians (Variables|Default|GetMesh) (Math|Vector|MakeVector (* (.x ActionValue) _acceleration) (* (.y ActionValue) _acceleration) 0.0) "None" true))

(event EventBeginPlay
  (Input|AddMappingContext (PlayerController|LocalPlayerSubsystems|GetEnhancedInputLocalPlayerSubsystem (Game|GetPlayerController 0)) "/Game/EnhancedInput/IMC_GameContext.IMC_GameContext" 0 "(bIgnoreAllPressedKeysUntilRelease=True,bForceImmediately=False,bNotifyUserSettings=False)")
  (CameraFades|StartCameraFade :self (Game|GetPlayerCameraManager 0) :FromAlpha 1.0 :Duration 1.0 :bHoldWhenFinished true))

(event Collision|EventActorBeginOverlap
  (params (OtherActor :type Actor%20Object%20Reference)))

(event EventTick
  (params (DeltaSeconds :type Float%20%28single-precision%29)))

(event Game|Damage|EventAnyDamage
  (params (Damage :type Float%20%28single-precision%29) (DamageType :type Damage%20Type%20Object%20Reference) (InstigatedBy :type Controller%20Object%20Reference) (DamageCauser :type Actor%20Object%20Reference))
  (Utilities|RestartLevel))

(fn ConstructionScript)